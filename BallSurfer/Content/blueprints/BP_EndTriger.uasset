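; Level-end trigger that lets the player advance only after every crystal is collected.
; On player pawn overlap with the Box, it checks for remaining BP_crystal actors and prints a Polish status message.
; If none remain, it opens the hard-coded Level02 after a short delay.
; Level-array helpers for next-level and last-level lookup exist but are not on the live path, and GetAllCrystals duplicates LadujemyTablice.
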(event `self.Box.OnComponentBeginOverlap`
  (params (OverlappedComponent :type "PrimitiveComponent Object Reference") (OtherActor :type "Actor Object Reference") (OtherComp :type "PrimitiveComponent Object Reference") (OtherBodyIndex :type Integer) (bFromSweep :type Boolean) (SweepResult :type "HitResult Structure (by ref)"))
  (if (== OtherActor (`GameplayStatics.GetPlayerPawn` 0))
    (bind _returnvalue (`self.LadujemyTablice`))
    (if _returnvalue
      (`KismetSystemLibrary.PrintString` "nie zebrales wszystkich krysztalow")
      (else
        (`KismetSystemLibrary.PrintString` "zebrales wszystkie krysztaly")
        (`KismetSystemLibrary.Delay` 0.2)
        (`GameplayStatics.OpenLevel` "Level02")))))

(event `self.ReceiveTick`
  (params (DeltaSeconds :type "Float (single-precision)")))

(fn `CheckLastLevel`
  (returns (`Return value` :type Boolean))
  (return (== (`self.GetCurrentLevelIndex`) (`KismetArrayLibrary.Array_LastIndex` (`self.ArrayLevelNames`)))))

(fn `GetAllCrystals`
  (returns (ReturnValue :type Boolean))
  (bind _outactors (`GameplayStatics.GetAllActorsOfClass` "/Game/blueprints/BP_crystal.BP_crystal_C"))
  (return (> (`KismetArrayLibrary.Array_Length` _outactors) 0)))

(fn `GetCurrentLevelIndex`
  (returns (NewParam :type Integer))
  (bind _returnvalue (`GameplayStatics.GetCurrentLevelName` true))
  (return (`KismetArrayLibrary.Array_Find` (`self.ArrayLevelNames`) (`KismetStringLibrary.Conv_StringToName` _returnvalue))))

(fn `LadujemyTablice`
  (returns (ReturnValue :type Boolean))
  (bind _outactors (`GameplayStatics.GetAllActorsOfClass` "/Game/blueprints/BP_crystal.BP_crystal_C"))
  (return (> (`KismetArrayLibrary.Array_Length` _outactors) 0)))

(fn `LoadNextindex`
  (returns (Output :type Name))
  (return (`|GetArrayItem` (`self.ArrayLevelNames`) (+ (`self.GetCurrentLevelIndex`) 1))))

(fn `UserConstructionScript`)