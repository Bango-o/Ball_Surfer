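; BP_crystal is a crystal actor that gets absorbed into the player pawn when the player overlaps its Sphere.
; The TL_crystal_gleam timeline drives helper functions that pull the crystal toward the player and shrink it to zero, while lerping down the PointLight intensity.
; Both helpers lerp from current values each update, so movement homes on a moving player and compounds.
; The actor destroys itself when the timeline finishes.
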(event `self.Sphere.OnComponentBeginOverlap`
  (params (OverlappedComponent :type "PrimitiveComponent Object Reference") (OtherActor :type "Actor Object Reference") (OtherComp :type "PrimitiveComponent Object Reference") (OtherBodyIndex :type Integer) (bFromSweep :type Boolean) (SweepResult :type "HitResult Structure (by ref)"))
  (if (== OtherActor (`GameplayStatics.GetPlayerPawn` 0))
    (bind (_direction _location_of_crystal _scale_of_crystal _light) (`Timeline|TL_crystal_gleam`)
      (:`Update`
        (`self.CrystalChangeLocation` _location_of_crystal)
        (`self.CrystalChangeScale` _scale_of_crystal)
        (`LightComponent.SetIntensity` (`self.PointLight`) (`KismetMathLibrary.Lerp` 2000.0 0.0 _light)))
      (:`Finished`
        (`self.K2_DestroyActor`)))))

(fn `CrystalChangeLocation`
  (params (alpha :type "Float (double-precision)"))
  (`self.K2_SetActorLocation` (`KismetMathLibrary.VLerp` (`self.K2_GetActorLocation`) (`self.K2_GetActorLocation` (`GameplayStatics.GetPlayerPawn` 0)) alpha)))

(fn `CrystalChangeScale`
  (params (Alpha :type "Float (double-precision)"))
  (`self.SetActorScale3D` (`KismetMathLibrary.VLerp` (`self.GetActorScale3D`) (0.0 0.0 0.0) Alpha)))

(fn `UserConstructionScript`)