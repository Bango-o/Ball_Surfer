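; BP_ball is a player-controlled rolling ball that restarts level01 when it takes damage.
; Both movement axes feed one AddTorqueInRadians call on the Sphere, applying the scaled value to X and Y together as an acceleration change.
; BeginPlay starts a camera fade-in; AnyDamage fades to black once, waits, then opens the level and destroys the actor.
; The ResetBall function is an empty stub.
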(event `InputAxis|MoveForwardBack`
  (params (AxisValue :type "Float (single-precision)"))
  (bind _strmultiply (`self.strmultiply`))
  (`PrimitiveComponent.AddTorqueInRadians` (`self.Sphere`) (`KismetMathLibrary.MakeVector` (* (stale `InputAxis|MoveLeftRight` AxisValue) _strmultiply) (* AxisValue _strmultiply)) "None" true :!label _label))

(event `InputAxis|MoveLeftRight`
  (params (AxisValue :type "Float (single-precision)"))
  (goto _label))

(event `self.ReceiveBeginPlay`
  (`PlayerCameraManager.StartCameraFade` :`self` (`GameplayStatics.GetPlayerCameraManager` 0) :`FromAlpha` 1.0 :`Duration` 5.0))

(event `self.ReceiveAnyDamage`
  (params (Damage :type "Float (single-precision)") (DamageType :type "DamageType Object Reference") (InstigatedBy :type "Controller Object Reference") (DamageCauser :type "Actor Object Reference"))
  (`/Engine/EditorBlueprintResources/StandardMacros.DoOnce` false
    (:`Completed`
      (`PlayerCameraManager.StartCameraFade` (`GameplayStatics.GetPlayerCameraManager` 0) 0.0 1.0 2.0 (struct :`A` 1.0) false true)
      (`KismetSystemLibrary.Delay` 2.0)
      (`GameplayStatics.OpenLevel` "level01")
      (`self.K2_DestroyActor`))))

(event `self.ReceiveTick`
  (params (DeltaSeconds :type "Float (single-precision)")))

(fn `Reset Ball`)

(fn `UserConstructionScript`)